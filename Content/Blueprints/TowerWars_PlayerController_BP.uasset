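; Player controller for the Tower Wars game, handling camera movement, unit selection and upgrade commands.
; Axis, speed-toggle, zoom and mouse screen-edge input are forwarded to a MovementComponent.
; Left click stores the selectable target as the selected actor and prints its type.
; Q sends an Upgrade command with the player state's gold to that actor and subtracts the returned cost.
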(event `InputAxis|MoveForward`
  (params (AxisValue :type "Float (single-precision)"))
  ;[1 1 1] Movement X
  (`CameraMovementComponent.MovementX` (`self.MovementComponent`) AxisValue))

(event `InputAxis|MoveRight`
  (params (AxisValue :type "Float (single-precision)"))
  ;[1 1 1] Movement Y
  (`CameraMovementComponent.MovementY` (`self.MovementComponent`) AxisValue))

(event `InputAction|ZoomIn`
  (params (Key :type "Key Structure"))
  ;[1 1 1] Zoom
  (:`Pressed`
    (`CameraMovementComponent.Zoom` (`self.MovementComponent`) true)))

(event `InputAction|FastMovement`
  (params (Key :type "Key Structure"))
  (bind _movementcomponent (`self.MovementComponent`))
  ;[1 1 1] Movement Multiplier
  (:`Pressed`
    (`CameraMovementComponent.ToggleMovementMultiplier` _movementcomponent true))
  (:`Released`
    (`CameraMovementComponent.ToggleMovementMultiplier` _movementcomponent false)))

(event `InputAction|ZoomOut`
  (params (Key :type "Key Structure"))
  ;[1 1 1] Zoom
  (:`Pressed`
    (`CameraMovementComponent.Zoom` (`self.MovementComponent`) false)))

(event `InputAxisKey|MouseX`
  (params (AxisValue :type "Float (single-precision)"))
  (bind (_locationx _locationy) (`self.GetMousePosition`))
  ;[1 1 1] Mouse Movement
  (`CameraMovementComponent.ScreenEdgeMovement` (`self.MovementComponent`) (`KismetMathLibrary.MakeVector2D` _locationx _locationy) (`WidgetLayoutLibrary.GetViewportSize`) :!label _label))

(event `InputAxisKey|MouseY`
  (params (AxisValue :type "Float (single-precision)"))
  ;[1 1 1] Mouse Movement
  (goto _label))

(event `Key|LeftMouseButton`
  (params (Key :type "Key Structure"))
  (bind _selectedactor (`self.SelectedActor`))
  (:`Pressed`
    (bind _returnvalue (`self.GetSelectableTarget`))
    (`self.SetSelectedActor` _returnvalue)
    (bind _returnvalue_2 (message `SelectionInterface.GetType` _selectedactor))
    (`KismetSystemLibrary.PrintString` (`KismetStringLibrary.Concat_StrStr` (`KismetSystemLibrary.GetDisplayName` _selectedactor) " of type " (`|GetEnumeratorNameAsString` _returnvalue_2)))))

(event `Key|Q`
  (params (Key :type "Key Structure"))
  (bind _astower_wars_player_state (cast `TowerWarsPlayerState` (`self.PlayerState`) :!pure true))
  (:`Pressed`
    (bind _returnvalue (message `CommandInterface.IssueCommand` (`self.SelectedActor`) "Upgrade" 0 (`TowerWarsPlayerState.Gold` _astower_wars_player_state)))
    (`TowerWarsPlayerState.IncrementGold` _astower_wars_player_state (* _returnvalue -1))))

(fn `UserConstructionScript`)