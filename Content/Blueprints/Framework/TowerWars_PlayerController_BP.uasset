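; Player controller for Tower Wars that drives the camera, actor selection and tower commands, and creates the HUD on BeginPlay.
; Axis, fast-move, zoom and mouse inputs are forwarded to a MovementComponent, with mouse movement feeding screen-edge scrolling.
; Left click stores the selectable target as the selected actor, while Q and Z issue non-sell and sell commands.
; A selected-actor type debug print is left unconnected.
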(event `InputAxis|MoveForward`
  (params (AxisValue :type "Float (single-precision)"))
  ;[1 1 1] Movement X
  (`CameraMovementComponent.MovementX` (`self.MovementComponent`) AxisValue))

(event `InputAxis|MoveRight`
  (params (AxisValue :type "Float (single-precision)"))
  ;[1 1 1] Movement Y
  (`CameraMovementComponent.MovementY` (`self.MovementComponent`) AxisValue))

(event `InputAction|ZoomIn`
  (params (Key :type "Key Structure"))
  ;[1 1 1] Zoom
  (:`Pressed`
    (`CameraMovementComponent.Zoom` (`self.MovementComponent`) true)))

(event `InputAction|FastMovement`
  (params (Key :type "Key Structure"))
  (bind _movementcomponent (`self.MovementComponent`))
  ;[1 1 1] Movement Multiplier
  (:`Pressed`
    (`CameraMovementComponent.ToggleMovementMultiplier` _movementcomponent true))
  (:`Released`
    (`CameraMovementComponent.ToggleMovementMultiplier` _movementcomponent false)))

(event `InputAction|ZoomOut`
  (params (Key :type "Key Structure"))
  ;[1 1 1] Zoom
  (:`Pressed`
    (`CameraMovementComponent.Zoom` (`self.MovementComponent`) false)))

(event `InputAxisKey|MouseX`
  (params (AxisValue :type "Float (single-precision)"))
  (bind (_locationx _locationy) (`self.GetMousePosition`))
  ;[1 1 1] Mouse Movement
  (`CameraMovementComponent.ScreenEdgeMovement` (`self.MovementComponent`) (`KismetMathLibrary.MakeVector2D` _locationx _locationy) (`WidgetLayoutLibrary.GetViewportSize`) :!label _label))

(event `InputAxisKey|MouseY`
  (params (AxisValue :type "Float (single-precision)"))
  ;[1 1 1] Mouse Movement
  (goto _label))

(event `Key|LeftMouseButton`
  (params (Key :type "Key Structure"))
  (:`Pressed`
    (bind _returnvalue (`self.GetSelectableTarget`))
    (`self.SetSelectedActor` _returnvalue)))

(event `Key|Q`
  (params (Key :type "Key Structure"))
  (:`Pressed`
    (`self.IssueCommand` "AnyButSell")))

(event `Key|Z`
  (params (Key :type "Key Structure"))
  (:`Pressed`
    (`self.IssueCommand` "Sell")))

(event `self.ReceiveBeginPlay`
  (bind _returnvalue (`|CreateWidget` "/Game/Blueprints/UI/HUD_BP.HUD_BP_C" self))
  (`UserWidget.AddToViewport` _returnvalue 0))

(fn `UserConstructionScript`)